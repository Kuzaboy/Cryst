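; NPC dialogue Blueprint that shows lines from a data table in a widget, advancing one line per interaction.
; BeginPlay builds a speaker queue from all rows and caches row names matching the location, dialogue number and either the player or this NPC.
; Interact increments the line index, then finds the cached row matching speaker, line and choice.
; Without exactly one match, it removes the widget and resets the index; debug prints remain throughout.
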(event EventBeginPlay
  (bind _outrownames (DataTable|GetDataTableRowNames "/Game/Blueprints/DialogueSys_-_Sheet1.DialogueSys_-_Sheet1"))
  (for _array_element _outrownames
    (bind _returnvalue (Utilities|GetDataTableRow "/Game/Blueprints/DialogueSys_-_Sheet1.DialogueSys_-_Sheet1" _array_element)
      (:then
        (if (Utilities|Enum|Equal(Enum) (.Character_D (Utilities|Struct|BreakDialogue_Structure _returnvalue)) (Variables|Default|GetPlayer))
          (Utilities|Array|Add (Variables|Default|GetDialogueQueue) (Utilities|String|StringToName (Variables|Default|GetPlayer)))
          (else
            (Utilities|Array|Add (Variables|Default|GetDialogueQueue) (Utilities|String|StringToName (Variables|Default|GetCharacter_D)))))
        (if (and (Class|KismetMathLibrary|XORBoolean (and (Utilities|Enum|Equal(Enum) (.Character_D (Utilities|Struct|BreakDialogue_Structure _returnvalue)) (Variables|Default|GetPlayer)) (Utilities|Enum|Equal(Enum) (.Location_D (Utilities|Struct|BreakDialogue_Structure _returnvalue)) (Variables|Default|GetLocation_D))) (and (Utilities|Enum|Equal(Enum) (.Character_D (Utilities|Struct|BreakDialogue_Structure _returnvalue)) (Variables|Default|GetCharacter_D)) (Utilities|Enum|Equal(Enum) (.Location_D (Utilities|Struct|BreakDialogue_Structure _returnvalue)) (Variables|Default|GetLocation_D)))) (== (.Nr_D (Utilities|Struct|BreakDialogue_Structure _returnvalue)) (Variables|Default|GetNR_D)))
          (Utilities|Array|Add (Variables|Default|GetRowNrText) _array_element)
          (Development|PrintString (Utilities|String|ToString(Name) _array_element) true true "(R=0.000000,G=0.660000,B=1.000000,A=1.000000)" 5e+01))))))

(event EventInteract
  (Math|Integer|IncrementInt (Variables|Default|GetLineCurrent)
    (:%20%20
      (CallFunction|DialogueCreate))))

(fn ConstructionScript)

(fn DialogueCreate
  (Utilities|IsValid (Variables|Default|GetDialogueWidget)
    (:Is%20Valid
      (bind _returnedline (CallFunction|DialogueGetLine))
      (Variables|/Game/Blueprints/W_Dialogue.W_Dialogue_C|SetTextDialogue (Variables|Default|GetDialogueWidget) _returnedline))
    (:Is%20Not%20Valid
      (bind _returnvalue (UserInterface|CreateWidget "/Game/Blueprints/W_Dialogue.W_Dialogue_C" (Game|GetPlayerController 0)))
      (bind _output_get (Variables|Default|SetDialogueWidget _returnvalue))
      (UserInterface|Viewport|AddtoViewport _output_get 0)
      (bind _returnedline_2 (CallFunction|DialogueGetLine))
      (Variables|/Game/Blueprints/W_Dialogue.W_Dialogue_C|SetTextDialogue (Variables|Default|GetDialogueWidget) _returnedline_2))))

(fn DialogueGetLine
  (for _array_element (Variables|Default|GetRowNrText)
    (bind _returnvalue (Utilities|GetDataTableRow "/Game/Blueprints/DialogueSys_-_Sheet1.DialogueSys_-_Sheet1" _array_element)
      (:then
        (Development|PrintString (Utilities|String|ToString(Name) (Utilities|Array|Get(acopy) (Variables|Default|GetDialogueQueue) (Variables|Default|GetLineCurrent))))
        (Development|PrintString (Utilities|String|ToString(Integer) (Variables|Default|GetLineCurrent)))
        (if (and (Utilities|Enum|Equal(Enum) (Utilities|String|ToString(Name) (Utilities|Array|Get(acopy) (Variables|Default|GetDialogueQueue) (Variables|Default|GetLineCurrent))) (.Character_D (Utilities|Struct|BreakDialogue_Structure _returnvalue))) (and (== (.Line_D (Utilities|Struct|BreakDialogue_Structure _returnvalue)) (Variables|Default|GetLineCurrent)) (== (.Сhoice_D (Utilities|Struct|BreakDialogue_Structure _returnvalue)) (Variables|Default|GetChoice_D))))
          (Utilities|Array|Add (LocalVariables|GetReturnedLines) (.Text_D (Utilities|Struct|BreakDialogue_Structure _returnvalue)))
          (Development|PrintString (Utilities|String|ToString(Text) (.Text_D (Utilities|Struct|BreakDialogue_Structure _returnvalue))))))))
  (if (== (Utilities|Array|Length (LocalVariables|GetReturnedLines)) 1)
    (return (Utilities|Array|Get(acopy) (LocalVariables|GetReturnedLines)))
    (else
      (Widget|RemovefromParent (Variables|Default|GetDialogueWidget))
      (Variables|Default|SetDialogueWidget 0)
      (Variables|Default|SetLineCurrent 0))))