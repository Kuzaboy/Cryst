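; Mr. Mutant NPC that acts as a dialogue participant, starting a conversation when the player walks into it.
; On overlap it casts to BP_Player and its BP_Mouse controller, then calls StartDialogue with its dialogue asset and itself.
; Participant functions supply its name, gender and speaker-based icon, while condition and value functions are default stubs.
; Dialogue color events only print debug strings.
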(event Collision|EventActorBeginOverlap
  (params (OtherActor :type Actor%20Object%20Reference))
  (bind _asbp_player (Utilities|Casting|CastToBP_Player OtherActor))
  (bind _asbp_mouse (Utilities|Casting|CastToBP_Mouse (Pawn|GetController _asbp_player)))
  (Default|StartDialogue _asbp_mouse (Variables|Default|GetDlgDialogue) self))

(fn ConstructionScript)

(fn CheckCondition
  (params (ConditionName :type Name%20%28by%20ref%29 :default "None"))
  (return false))

(fn GetBoolValue
  (params (ValueName :type Name%20%28by%20ref%29 :default "None"))
  (return false))

(fn GetFloatValue
  (params (ValueName :type Name%20%28by%20ref%29 :default "None"))
  (return 0.0))

(fn GetIntValue
  (params (ValueName :type Name%20%28by%20ref%29 :default "None"))
  (return 0))

(fn GetNameValue
  (params (ValueName :type Name%20%28by%20ref%29 :default "None"))
  (return "None"))

(fn GetParticipantDisplayName
  (params (ActiveSpeaker :type Name :default "None"))
  (return ""))

(fn GetParticipantGender
  (return "Masculine"))

(fn GetParticipantIcon
  (params (ActiveSpeaker :type Name :default "None") (ActiveSpeakerState :type Name :default "None"))
  (return (|SelectonSpeakerState ActiveSpeaker (Variables|Default|GetActiveIcon) "/Game/Blueprints/Dialogue_System/Icons/Rock_Slime.Rock_Slime")))

(fn GetParticipantName
  (return (Variables|Default|GetMyName)))

(fn ModifyBoolValue
  (params (ValueName :type Name%20%28by%20ref%29 :default "None") (bNewValue :type Boolean))
  (return false))

(fn ModifyFloatValue
  (params (ValueName :type Name%20%28by%20ref%29 :default "None") (bDelta :type Boolean) (Value :type Float%20%28single-precision%29))
  (return false))

(fn ModifyIntValue
  (params (ValueName :type Name%20%28by%20ref%29 :default "None") (bDelta :type Boolean) (Value :type Integer))
  (return false))

(fn ModifyNameValue
  (params (ValueName :type Name%20%28by%20ref%29 :default "None") (NameValue :type Name%20%28by%20ref%29 :default "None"))
  (return false))

(fn OnDialogueEvent
  (params (EventName :type Name%20%28by%20ref%29 :default "None"))
  (|SwitchDialogueCallbackEvent EventName
    (:Default
      (return false))
    (:ColorToBlue
      (Development|PrintString "BLUE!"))
    (:ColorToGreen
      (Development|PrintString "GREEN!"))
    (:ColorToRed
      (Development|PrintString "RED!")))
  (return false))