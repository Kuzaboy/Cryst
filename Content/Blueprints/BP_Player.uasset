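; Player character Blueprint for control-rotation-relative movement with keyboard and gamepad, walking while Left Shift or the bottom face button is held.
; Tick picks walk or run Speed from NewVar0, which scales the MoveForward and MoveRight inputs.
; For keyboard input, flagged by the isKeyboard axis, Speed drops to 0.71 when IsAngle is set, compensating for diagonals.
; Tick also prints movement state and velocity on screen for debugging.
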(event EventTick
  (params (DeltaSeconds :type Float%20%28single-precision%29))
  (bind _newvar_0 (Variables|Default|GetNewVar_0))
  (bind _newvar_0_2 (Variables|Default|GetNewVar_0))
  (bind (_speedwalk _speedrun) (Utilities|Struct|BreakStr_DefVarPlayer _newvar_0_2))
  (bind (_speedwalk_2 _speedrun_2) (Utilities|Struct|BreakStr_DefVarPlayer _newvar_0))
  (Utilities|FlowControl|Sequence
    (:then_0
      (Variables|Default|SetisAngle (Math|Boolean|Equal(Boolean) (!= (stale Input|AxisEvents|InputAxisMoveForward AxisValue) 0.0) (!= (stale Input|AxisEvents|InputAxisMoveRight AxisValue) 0.0))))
    (:then_1
      (Development|PrintString (Utilities|String|Append (Utilities|String|MakeLiteralString "Keyboard: ") (Utilities|String|ToString(Boolean) (Variables|Default|GetisKeyboard))) true true "(R=0.290336,G=0.693796,B=0.770833,A=1.000000)" 0.0)
      (Development|PrintString (Utilities|String|Append (Utilities|String|MakeLiteralString "Velocity: ") (Utilities|String|ToString(Float) (Math|Vector|VectorLength (Variables|/Script/Engine.MovementComponent|GetVelocity (Variables|Character|GetCharacterMovement))))) true true "(R=0.538863,G=1.000000,B=0.510860,A=1.000000)" 0.0)
      (Development|PrintString (Utilities|String|ToString(Vector) (Class|Pawn|GetLastMovementInputVector)) true true "(R=1.000000,G=0.336433,B=0.862252,A=1.000000)" 0.0)
      (Development|PrintString (Utilities|String|Append (Utilities|String|MakeLiteralString "Is Walking: ") (Utilities|String|ToString(Boolean) (Variables|Default|GetisWalking))) true true "(R=0.290336,G=0.693796,B=0.770833,A=1.000000)" 0.0)
      (Development|PrintString (Utilities|String|Append (Utilities|String|MakeLiteralString "Is Angle: ") (Utilities|String|ToString(Boolean) (Variables|Default|GetisAngle))) true true "(R=0.290336,G=0.693796,B=0.770833,A=1.000000)" 0.0))
    (:then_2
      (if (Variables|Default|GetisKeyboard)
        (if (Variables|Default|GetisAngle)
          (if (Variables|Default|GetisWalking)
            (Variables|Default|Setspeed (* _speedwalk_2 0.71))
            (else
              (Variables|Default|Setspeed (* _speedrun_2 0.71))))
          (else
            (if (Variables|Default|GetisWalking) :!label _label
              (Variables|Default|Setspeed _speedwalk)
              (else
                (Variables|Default|Setspeed _speedrun)))))
        (else
          (goto _label))))))

(event Input|AxisEvents|InputAxisisKeyboard
  (params (AxisValue :type Float%20%28single-precision%29))
  (Variables|Default|SetisKeyboard (> AxisValue 0.0)))

(event Input|AxisEvents|InputAxisMoveRight
  (params (AxisValue :type Float%20%28single-precision%29))
  (Pawn|Input|AddMovementInput (Math|Vector|GetRightVector (Pawn|GetControlRotation :!class /Script/Engine.Pawn)) (* AxisValue (Variables|Default|Getspeed)) false))

(event Input|AxisEvents|InputAxisMoveForward
  (params (AxisValue :type Float%20%28single-precision%29))
  (Pawn|Input|AddMovementInput (Math|Vector|GetForwardVector (Pawn|GetControlRotation :!class /Script/Engine.Pawn)) (* AxisValue (Variables|Default|Getspeed)) false))

(event Input|KeyboardEvents|LeftShift
  (params (Key :type Key%20Structure))
  (:Pressed
    (Variables|Default|SetisWalking true))
  (:Released
    (Variables|Default|SetisWalking false)))

(event Input|GamepadEvents|GamepadFaceButtonBottom
  (params (Key :type Key%20Structure))
  (:Pressed
    (Variables|Default|SetisWalking true))
  (:Released
    (Variables|Default|SetisWalking false)))

(fn ConstructionScript)