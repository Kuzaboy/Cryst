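; BP_mouse is a Blueprint that starts and drives branching dialogue between another participant and the player pawn.
; StartDialogue creates a two-participant dialogue context and stores it as ActiveContext.
; SelectDialogueOption validates the context and option index, advances through the chosen child, and clears ActiveContext when that call returns false.
; The event graph and construction script hold no logic.
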(event EventBeginPlay)

(event EventTick
  (params (DeltaSeconds :type Float%20%28single-precision%29)))

(fn ConstructionScript)

(fn StartDialogue
  (params (Dialogue :type Dlg%20Dialogue%20Object%20Reference) (OtherParticipant :type Object%20Object%20Reference))
  (bind _returnvalue (Class|DlgManager|StartDialogue2 Dialogue OtherParticipant (Game|Player|GetPlayerPawn 0)))
  (Variables|Default|SetActiveContext _returnvalue))

(fn SelectDialogueOption
  (params (OptionIndex :type Integer))
  (Utilities|IsValid (Variables|Default|GetActiveContext)
    (:Is%20Valid
      (if (and (< OptionIndex (Class|DlgContext|GetOptionNum (Variables|Default|GetActiveContext))) (> OptionIndex -1))
        (bind _returnvalue (Class|DlgContext|ChooseChild (Variables|Default|GetActiveContext) OptionIndex))
        (if (not _returnvalue)
          (Variables|Default|SetActiveContext 0))))))