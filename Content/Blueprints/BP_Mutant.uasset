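; BP_Mutant is an interactable mutant that shows a line of dialogue on screen.
; Its Interact event toggles a W_Dialogue widget, removing and clearing it if open, otherwise creating it for the first player controller.
; The new widget is added to the viewport, then receives the mutant's MyText as its TextDialogue.
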(event EventInteract
  (Utilities|IsValid (Variables|Default|GetDialogueWidget)
    (:Is%20Valid
      (Widget|RemovefromParent (Variables|Default|GetDialogueWidget))
      (Variables|Default|SetDialogueWidget 0))
    (:Is%20Not%20Valid
      (bind _returnvalue (UserInterface|CreateWidget "/Game/Blueprints/W_Dialogue.W_Dialogue_C" (Game|GetPlayerController 0)))
      (bind _output_get (Variables|Default|SetDialogueWidget _returnvalue))
      (UserInterface|Viewport|AddtoViewport _output_get 0)
      (Variables|/Game/Blueprints/W_Dialogue.W_Dialogue_C|SetTextDialogue (Variables|Default|GetDialogueWidget) (Variables|Default|GetMyText)))))

(fn ConstructionScript)